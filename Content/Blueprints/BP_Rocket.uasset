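; Rocket projectile actor that explodes on contact and destroys itself five seconds after spawning.
; Its box overlap spawns an explosion particle and sound, then destroys the other actor if tagged "Item".
; After the self-destroy call, BeginPlay line-traces to "Enemy" actors to pick a nearest Target.
; That distance test requires a value below zero, so Target is never set, and nothing here reads it.
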(event `self.ReceiveBeginPlay`
  (`KismetSystemLibrary.Delay` 5.0)
  (`self.K2_DestroyActor`)
  (bind _outactors (`GameplayStatics.GetAllActorsWithTag` "Enemy"))
  (for _array_element _outactors
    (bind _outhit (`KismetSystemLibrary.LineTraceSingle` :`Start` (`self.K2_GetActorLocation`) :`End` (`self.K2_GetActorLocation` _array_element) :`TraceChannel` "TraceTypeQuery1" :`DrawDebugType` "ForDuration"))
    (bind (_bblockinghit _binitialoverlap _time _distance _location _impactpoint _normal _impactnormal _physmat _hitactor _hitcomponent _hitbonename _hititem _elementindex _faceindex _tracestart _traceend) (`GameplayStatics.BreakHitResult` _outhit))
    (bind _returnvalue (`KismetMathLibrary.Vector_GetAbs` (- _tracestart _traceend)))
    (if (< (`KismetMathLibrary.Vector_Distance` (- (`self.MinVector`) _returnvalue) _returnvalue) 0.0)
      (set `self.MinVector` _returnvalue)
      (set `self.target` _hitactor))))

(event `self.Box.OnComponentBeginOverlap`
  (params (OverlappedComponent :type "PrimitiveComponent Object Reference") (OtherActor :type "Actor Object Reference") (OtherComp :type "PrimitiveComponent Object Reference") (OtherBodyIndex :type Integer) (bFromSweep :type Boolean) (SweepResult :type "HitResult Structure (by ref)"))
  (bind (_returnvalue_location _returnvalue_rotation _returnvalue_scale) (`KismetMathLibrary.BreakTransform` (`SceneComponent.K2_GetComponentToWorld` OverlappedComponent)))
  (`GameplayStatics.SpawnEmitterAtLocation` "/Game/StarterContent/Particles/P_Explosion.P_Explosion" _returnvalue_location _returnvalue_rotation _returnvalue_scale)
  (`GameplayStatics.PlaySoundAtLocation` "/Game/StarterContent/Audio/Explosion_Cue.Explosion_Cue" _returnvalue_location (struct) 1.0 1.0 0.0 null null null)
  (if (`self.ActorHasTag` OtherActor "Item")
    (`self.K2_DestroyActor` OtherActor)))

(fn `UserConstructionScript`)