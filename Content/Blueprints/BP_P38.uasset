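; BP_P38 is a player-controlled P-38 aircraft pawn with twin spinning propellers and rocket firing.
; Clamped yaw, roll and pitch axes drive controller rotation input, while the forward movement call is left disconnected.
; Tick spins both propellers through a shared RotatePropeller function scaled by delta time and RotationSpeed.
; The SpawnRocket action spawns a BP_Rocket at both the left and right spawn transforms on each press.
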(event `InputAxis|YAw`
  (params (AxisValue :type "Float (single-precision)"))
  ;[1 1 1] Yaw
  (`self.AddControllerYawInput` (`KismetMathLibrary.FClamp` AxisValue -1.0)))

(event `InputAxis|Roll`
  (params (AxisValue :type "Float (single-precision)"))
  ;[1 1 1] Roll
  (`self.AddControllerRollInput` (`KismetMathLibrary.FClamp` AxisValue -1.0)))

(event `InputAxis|Pitch`
  (params (AxisValue :type "Float (single-precision)"))
  ;[1 1 1] Pitch
  (`self.AddControllerPitchInput` (`KismetMathLibrary.FClamp` AxisValue -1.0)))

(event `self.ReceiveTick`
  (params (DeltaSeconds :type "Float (single-precision)"))
  ;[1 1 1] RightPropellerRotate
  (`self.RotatePropeller` (`self.RightPropeller`))
  ;[1 1 1] LeftPropellerRotate
  (`self.RotatePropeller` (`self.LefttPropeller`)))

(event `InputAction|SpawnRocket`
  (params (Key :type "Key Structure"))
  (:`Pressed`
    (`|SpawnActorFromClass` "/Game/Blueprints/BP_Rocket.BP_Rocket_C" (`SceneComponent.K2_GetComponentToWorld` (`self.RightRocketSpawnTransform`)) "Undefined" "OverrideRootScale" null null)
    (`|SpawnActorFromClass` "/Game/Blueprints/BP_Rocket.BP_Rocket_C" (`SceneComponent.K2_GetComponentToWorld` (`self.LefttRocketSpawnTransform`)) "Undefined" "OverrideRootScale" null null)))

(fn `RotatePropeller`
  (params (self2 :type "SceneComponent Object Reference"))
  (`SceneComponent.K2_AddLocalRotation` self2 (`KismetMathLibrary.MakeRotator` (* (`GameplayStatics.GetWorldDeltaSeconds`) (`self.RotationSpeed`))) false false))

(fn `UserConstructionScript`)